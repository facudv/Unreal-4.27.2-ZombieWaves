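; BP_Zombie is a zombie enemy Blueprint that wires its components into enemy logic defined outside its graphs.
; On BeginPlay it links itself to the LifeBar widget, sets the spit spawn point and stores its colliders in variables.
; Sphere overlaps feed begin and end handlers for obstacle avoidance.
; Body and arm collider overlaps call BodyCollisionHandler with a body-part index for per-part score and damage.
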(event OnComponentBeginOverlap(Sphere)
  (params (OverlappedComponent :type Primitive%20Component%20Object%20Reference) (OtherActor :type Actor%20Object%20Reference) (OtherComp :type Primitive%20Component%20Object%20Reference) (OtherBodyIndex :type Integer) (bFromSweep :type Boolean) (SweepResult :type Hit%20Result%20Structure%20%28by%20ref%29))
  ;[0.4862 1 0.4456] Obstacle Avoidance
  (Class|Zombie|MyBeginOverlap OtherActor))

(event OnComponentEndOverlap(Sphere)
  (params (OverlappedComponent :type Primitive%20Component%20Object%20Reference) (OtherActor :type Actor%20Object%20Reference) (OtherComp :type Primitive%20Component%20Object%20Reference) (OtherBodyIndex :type Integer))
  ;[0.4862 1 0.4456] Obstacle Avoidance
  (Class|Zombie|MyEndOverlap OtherActor))

(event OnComponentBeginOverlap(armcolliderR)
  (params (OverlappedComponent :type Primitive%20Component%20Object%20Reference) (OtherActor :type Actor%20Object%20Reference) (OtherComp :type Primitive%20Component%20Object%20Reference) (OtherBodyIndex :type Integer) (bFromSweep :type Boolean) (SweepResult :type Hit%20Result%20Structure%20%28by%20ref%29))
  ;[1 0.4896 0.4896] Puntaje y Daño por Parte del cuerpo
  (Class|Zombie|BodyCollisionHandler OtherActor 2))

(event OnComponentBeginOverlap(armcolliderL)
  (params (OverlappedComponent :type Primitive%20Component%20Object%20Reference) (OtherActor :type Actor%20Object%20Reference) (OtherComp :type Primitive%20Component%20Object%20Reference) (OtherBodyIndex :type Integer) (bFromSweep :type Boolean) (SweepResult :type Hit%20Result%20Structure%20%28by%20ref%29))
  ;[1 0.4896 0.4896] Puntaje y Daño por Parte del cuerpo
  (Class|Zombie|BodyCollisionHandler OtherActor 1))

(event OnComponentBeginOverlap(zombieArea)
  (params (OverlappedComponent :type Primitive%20Component%20Object%20Reference) (OtherActor :type Actor%20Object%20Reference) (OtherComp :type Primitive%20Component%20Object%20Reference) (OtherBodyIndex :type Integer) (bFromSweep :type Boolean) (SweepResult :type Hit%20Result%20Structure%20%28by%20ref%29))
  ;[1 0.4896 0.4896] Puntaje y Daño por Parte del cuerpo
  (Class|Zombie|BodyCollisionHandler OtherActor))

(event EventBeginPlay
  (bind _output_get (Variables|Default|SetlifeBarWidget (UserInterface|GetUserWidgetObject (Variables|Default|GetLifeBar))))
  (bind _aslife_bar (Utilities|Casting|CastToLifeBar _output_get))
  (bind _output_get_2 (Variables|/Game/Blueprints/UI/LifeBar.LifeBar_C|SetEnemy _aslife_bar self))
  (Variables|/Script/ZombieGame.Zombie|SetSpitSpawner _output_get_2 (Variables|Default|GetSpitSpawnPosition))
  (Variables|Default|SetmyBoxCollider1 (Variables|Default|GetarmcolliderR))
  (Variables|Default|SetmyBoxCollider2 (Variables|Default|GetarmcolliderL))
  (Variables|Default|SetmySphereCollider (Variables|Default|GetSphere))
  (Variables|Default|SetmyCapsuleCollider (Variables|Default|GetzombieArea)))

(event Collision|EventActorBeginOverlap
  (params (OtherActor :type Actor%20Object%20Reference)))

(fn ConstructionScript)